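; BP_CustomLighting feeds a custom light position and direction, taken from its Arrow component, into the CharacterCustomCollection material parameter collection.
; On BeginPlay a looping timer at the TimerUpdate interval runs RefreshLight instead of updating every frame.
; RefreshLight writes the Arrow's world location as LightPosition and its negated forward vector as LightDirection.
; The construction script also writes LightDirection, but leaves LightPosition to the timer.
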(event Custom|RefreshLight
  ;[1 1 1] Useing a timer to not tick every frame
  (Rendering|Material|SetVectorParameterValue (Variables|Default|GetCharacterCustomCollection) (Utilities|Name|MakeLiteralName "LightPosition") (Math|Conversions|ToLinearColor(Vector) (Transformation|GetWorldLocation (Variables|Default|GetArrow))) :!class /Script/Engine.KismetMaterialLibrary)
  (Rendering|Material|SetVectorParameterValue (Variables|Default|GetCharacterCustomCollection) (Utilities|Name|MakeLiteralName "LightDirection") (Math|Conversions|ToLinearColor(Vector) (* (Math|Vector|GetForwardVector (Variables|Default|GetArrow)) -1.0)) :!class /Script/Engine.KismetMaterialLibrary))

(event EventBeginPlay
  ;[1 1 1] Useing a timer to not tick every frame
  (Utilities|Time|SetTimerbyEvent (delegate Custom|RefreshLight) (Variables|Default|GetTimerUpdate) true))

(event EventTick
  (params (DeltaSeconds :type Float%20%28single-precision%29)))

(fn ConstructionScript
  (Rendering|Material|SetVectorParameterValue (Variables|Default|GetCharacterCustomCollection) (Utilities|Name|MakeLiteralName "LightDirection") (Math|Conversions|ToLinearColor(Vector) (* (Math|Vector|GetForwardVector (Variables|Default|GetArrow)) -1.0)) :!class /Script/Engine.KismetMaterialLibrary))