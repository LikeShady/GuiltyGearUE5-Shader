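; BP_CharacterBase is a character base that drives custom shading on its meshes according to whether it is occluded from a light.
; A looping timer traces from the actor to the collection's LightPosition and interpolates CurrentShade toward the hit result.
; It writes Shade to MeshToShade materials, plus LightDirection when UseCustomLighting is set, which the construction script also applies.
; The trace still has debug drawing and printing enabled.
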(event Custom|SetShade
  (bind _returnvalue (Rendering|Material|GetVectorParameterValue (Variables|/Game/BP/BP_CustomLighting.BP_CustomLighting_C|GetCharacterCustomCollection (Variables|Lighting|GetCustomLightingRef)) (Utilities|Name|MakeLiteralName "LightPosition") :!class /Script/Engine.KismetMaterialLibrary))
  (CallFunction|CheckShade _returnvalue)
  (CallFunction|SetShadeMaterial (Variables|Default|GetMeshToShade))
  (if (Variables|Lighting|GetUseCustomLighting)
    (CallFunction|CustomLightDirection)))

(event EventBeginPlay
  (Utilities|Time|SetTimerbyEvent (delegate Custom|SetShade) (Variables|Default|GetTimeForShade) true))

(fn ConstructionScript
  (if (Variables|Lighting|GetUseCustomLighting)
    (CallFunction|CustomLightDirection)))

(fn SetShadeMaterial
  (params (MeshToShade :type Array%20of%20Mesh%20Component%20Object%20References))
  (for _array_element MeshToShade
    (Rendering|Material|SetScalarParameterValueonMaterials _array_element "Shade" (Variables|Default|GetCurrentShade))))

(fn SetMeshtoShade
  (params (MeshToShade :type Array%20of%20Mesh%20Component%20Object%20References))
  (Variables|Default|SetMeshToShade MeshToShade))

(fn CustomLightDirection
  (bind _returnvalue (Rendering|Material|GetVectorParameterValue (Variables|/Game/BP/BP_CustomLighting.BP_CustomLighting_C|GetCharacterCustomCollection (Variables|Lighting|GetCustomLightingRef)) (Utilities|Name|MakeLiteralName "LightDirection") :!class /Script/Engine.KismetMaterialLibrary))
  (Variables|Lighting|SetLightDirection _returnvalue)
  (for _array_element (Variables|Default|GetMeshToShade)
    (Rendering|Material|SetVectorParameterValueonMaterials _array_element "LightDirection" (Math|Conversions|ToVector(LinearColor) (Variables|Lighting|GetLightDirection)))))

(fn CheckShade
  (params (LightPosition :type Linear%20Color%20Structure))
  (bind _returnvalue (Collision|LineTraceByChannel (Transformation|GetActorLocation) (* LightPosition 1.0) "TraceTypeQuery1" true 0 "ForDuration" true "(R=1.000000,G=0.000000,B=0.000000,A=1.000000)" "(R=0.000000,G=1.000000,B=0.000000,A=1.000000)" 1.0))
  (Development|PrintString (Utilities|String|ToString(Boolean) _returnvalue))
  (bind _output_get (Variables|Default|SetCurrentShade (Math|Interpolation|FInterpTo (Variables|Default|GetCurrentShade) (Math|Conversions|ToFloat(Boolean) _returnvalue) (Variables|Default|GetTimeForShade) 3.0)))
  (return _output_get))